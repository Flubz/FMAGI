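; BP_MainCharacter is the main character Blueprint, which switches the character's mining animation state with fire input events.
; OnFire and OnFireStop set the IsMining flag on ABP_Character to true and false.
; Both reach the Animation Blueprint through GetABP, a helper that casts and validates the mesh's anim instance.
; OnPlace is an empty stub.
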(event Custom|OnPlace)

(event Custom|OnFireStop
  (bind _asabp_character (CallFunction|GetABP))
  (Variables|/Game/_Flubz/Character/ABP_Character.ABP_Character_C|SetIsMining _asabp_character false))

(event Custom|OnFire
  (bind _asabp_character (CallFunction|GetABP))
  (Variables|/Game/_Flubz/Character/ABP_Character.ABP_Character_C|SetIsMining _asabp_character true))

(fn ConstructionScript)

(fn GetABP
  (bind _asabp_character (Utilities|Casting|CastToABP_Character (Components|SkeletalMesh|GetAnimInstance (Variables|Character|GetMesh))))
  (Utilities|IsValid _asabp_character
    (:Is%20Valid
      (return _asabp_character))))