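; Player controller that turns Fire, Place and Pause input into character actions, voxel edits and menu changes.
; Fire and Place notify the main character pawn, looked up for player 0, and call UpdateVoxel with a flag distinguishing the two, while releasing Fire stops firing.
; Pause switches the menu state machine on the game instance (BP_MenuManager) to its Pause state.
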(event Input|ActionEvents|InputActionFire
  (params (Key :type Key%20Structure))
  (:Pressed
    (bind _asbp_main_character (CallFunction|GetMainCharacter))
    (Utilities|IsValid _asbp_main_character
      (:Is%20Valid
        (Default|OnFire _asbp_main_character)
        (Class|MainPlayerController|UpdateVoxel false))))
  (:Released
    (bind _asbp_main_character_2 (CallFunction|GetMainCharacter))
    (Utilities|IsValid _asbp_main_character_2
      (:Is%20Valid
        (Default|OnFireStop _asbp_main_character_2)))))

(event Input|ActionEvents|InputActionPlace
  (params (Key :type Key%20Structure))
  (:Pressed
    (bind _asbp_main_character (CallFunction|GetMainCharacter))
    (Utilities|IsValid _asbp_main_character
      (:Is%20Valid
        (Default|OnPlace _asbp_main_character)
        (Class|MainPlayerController|UpdateVoxel true)))))

(event Input|ActionEvents|InputActionPause
  (params (Key :type Key%20Structure))
  (:Pressed
    (bind _asbp_menu_manager (Utilities|Casting|CastToBP_MenuManager (Game|GetGameInstance)))
    (Class|MenuStateMachine|SetState (Variables|/Script/FMAGI.MenuManager|Get_menuStateMachine _asbp_menu_manager) "Pause")))

(fn ConstructionScript)

(fn GetMainCharacter
  (bind _asbp_main_character (Utilities|Casting|CastToBP_MainCharacter (Game|Player|GetPlayerPawn 0))
    (:then
      (Utilities|IsValid _asbp_main_character
        (:Is%20Valid
          _)))
    (:CastFailed
      _))
  (return _asbp_main_character))