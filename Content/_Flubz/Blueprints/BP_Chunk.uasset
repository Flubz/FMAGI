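; BP_Chunk is a voxel chunk that holds grass and crystal blocks as instanced static meshes.
; AddInstanceVoxel places an instance at a given location, choosing crystal when GetCanSpawnCrystal allows it and grass otherwise.
; Overlapping a crystal removes an instance by the sweep hit item and sets the game instance's menu state machine to GameWon.
; Grass overlap does nothing, as its instance removal is disconnected.
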(event OnComponentBeginOverlap(ISM_Grass)
  (params (OverlappedComponent :type Primitive%20Component%20Object%20Reference) (OtherActor :type Actor%20Object%20Reference) (OtherComp :type Primitive%20Component%20Object%20Reference) (OtherBodyIndex :type Integer) (bFromSweep :type Boolean) (SweepResult :type Hit%20Result%20Structure%20%28by%20ref%29)))

(event OnComponentBeginOverlap(ISM_Crystal)
  (params (OverlappedComponent :type Primitive%20Component%20Object%20Reference) (OtherActor :type Actor%20Object%20Reference) (OtherComp :type Primitive%20Component%20Object%20Reference) (OtherBodyIndex :type Integer) (bFromSweep :type Boolean) (SweepResult :type Hit%20Result%20Structure%20%28by%20ref%29))
  (Class|InstancedStaticMeshComponent|RemoveInstance (Variables|Default|GetISM_Crystal) (.HitItem (Collision|BreakHitResult SweepResult)))
  (bind _asbp_menu_manager (Utilities|Casting|CastToBP_MenuManager (Game|GetGameInstance)))
  (Class|MenuStateMachine|SetState (Variables|/Script/FMAGI.MenuManager|Get_menuStateMachine _asbp_menu_manager) "GameWon"))

(event EventAddInstanceVoxel
  (params (instanceLocation :type Vector :default "0, 0, 0"))
  (bind _returnvalue (Math|Conversions|ToTransform(Vector) instanceLocation))
  (bind _returnvalue_2 (Class|Chunk|GetCanSpawnCrystal))
  (if _returnvalue_2
    (Components|InstancedStaticMesh|AddInstance (Variables|Default|GetISM_Crystal) _returnvalue)
    (else
      (Components|InstancedStaticMesh|AddInstance (Variables|Components|GetISM_Grass) _returnvalue))))

(fn ConstructionScript)